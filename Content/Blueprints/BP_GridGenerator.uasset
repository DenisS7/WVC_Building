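; Grid generator actor that visualizes a base quad grid as blue wireframe lines when its construction script runs.
; CreateFirstMeshGrid walks BaseGridQuads and BaseGridPoints, adding a shadowless cube component per edge, placed at the midpoint, rotated and stretched between endpoints.
; CreateSecondMeshGrid does the same for building grid shapes, but its calls are disconnected.
; Construction also gives HoveredShapeMesh a transparent gray material; BeginPlay and Tick do nothing.
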(event EventBeginPlay)

(event EventTick
  (params (DeltaSeconds :type Float%20%28single-precision%29)))

(fn ConstructionScript
  (|CallParentFunction)
  (CallFunction|CreateFirstMeshGrid)
  (Rendering|Material|SetMaterial (Variables|Default|GetHoveredShapeMesh) 0 "/Game/Assets/Material/MI_GrayTransparent.MI_GrayTransparent"))

(fn CreateSecondMeshGrid
  (for _array_element (Variables|Default|GetBuildingGridShapes)
    (for (_array_element_2 _array_index) (.Points (Utilities|Struct|BreakGridShape _array_element))
      (LocalVariables|SetPointIndex _array_element_2)
      (LocalVariables|SetNextPointIndex (Utilities|Array|Get(acopy) (.Points (Utilities|Struct|BreakGridShape _array_element)) (Math|Integer|%(Integer) (+ _array_index 1) (Utilities|Array|Length (.Points (Utilities|Struct|BreakGridShape _array_element))))))
      (bind _returnvalue (AddComponent|AddStaticMeshComponent false (Math|Transform|MakeTransform (- (/ (+ (.Location (Utilities|Struct|BreakGridPoint (Utilities|Array|Get(acopy) (Variables|Default|GetBuildingGridPoints) (LocalVariables|GetPointIndex)))) (.Location (Utilities|Struct|BreakGridPoint (Utilities|Array|Get(acopy) (Variables|Default|GetBuildingGridPoints) (LocalVariables|GetNextPointIndex))))) 2.0) (Transformation|GetActorLocation)) (Math|Rotator|FindLookatRotation (.Location (Utilities|Struct|BreakGridPoint (Utilities|Array|Get(acopy) (Variables|Default|GetBuildingGridPoints) (LocalVariables|GetPointIndex)))) (.Location (Utilities|Struct|BreakGridPoint (Utilities|Array|Get(acopy) (Variables|Default|GetBuildingGridPoints) (LocalVariables|GetNextPointIndex))))) (Math|Vector|MakeVector (/ (Math|Vector|Distance(Vector) (.Location (Utilities|Struct|BreakGridPoint (Utilities|Array|Get(acopy) (Variables|Default|GetBuildingGridPoints) (LocalVariables|GetPointIndex)))) (.Location (Utilities|Struct|BreakGridPoint (Utilities|Array|Get(acopy) (Variables|Default|GetBuildingGridPoints) (LocalVariables|GetNextPointIndex))))) 2.5e+02) 0.025 0.025))))
      (Components|StaticMesh|SetStaticMesh _returnvalue "/Engine/EngineMeshes/Cube.Cube")
      (Rendering|SetCastShadow _returnvalue false)
      (Rendering|Material|SetMaterial _returnvalue 0 "/Game/Assets/Material/MI_Blue.MI_Blue"))))

(fn CreateFirstMeshGrid
  (for _array_element (Variables|Default|GetBaseGridQuads)
    (for (_array_element_2 _array_index) (.Points (Utilities|Struct|BreakGridQuad _array_element))
      (LocalVariables|SetPointIndex _array_element_2)
      (LocalVariables|SetNextPointIndex (Utilities|Array|Get(acopy) (.Points (Utilities|Struct|BreakGridQuad _array_element)) (Math|Integer|%(Integer) (+ _array_index 1) (Utilities|Array|Length (.Points (Utilities|Struct|BreakGridQuad _array_element))))))
      (bind _returnvalue (AddComponent|AddStaticMeshComponent false (Math|Transform|MakeTransform (Utilities|Operators|Subtract (/ (+ (.Location (Utilities|Struct|BreakGridPoint (Utilities|Array|Get(acopy) (Variables|Default|GetBaseGridPoints) (LocalVariables|GetPointIndex)))) (.Location (Utilities|Struct|BreakGridPoint (Utilities|Array|Get(acopy) (Variables|Default|GetBaseGridPoints) (LocalVariables|GetNextPointIndex))))) 2.0) (Transformation|GetActorLocation) "0.000000,0.000000,-5.000000") (Math|Rotator|FindLookatRotation (.Location (Utilities|Struct|BreakGridPoint (Utilities|Array|Get(acopy) (Variables|Default|GetBaseGridPoints) (LocalVariables|GetPointIndex)))) (.Location (Utilities|Struct|BreakGridPoint (Utilities|Array|Get(acopy) (Variables|Default|GetBaseGridPoints) (LocalVariables|GetNextPointIndex))))) (Math|Vector|MakeVector (/ (Math|Vector|Distance(Vector) (.Location (Utilities|Struct|BreakGridPoint (Utilities|Array|Get(acopy) (Variables|Default|GetBaseGridPoints) (LocalVariables|GetPointIndex)))) (.Location (Utilities|Struct|BreakGridPoint (Utilities|Array|Get(acopy) (Variables|Default|GetBaseGridPoints) (LocalVariables|GetNextPointIndex))))) 2.5e+02) 0.025 0.025))))
      (Components|StaticMesh|SetStaticMesh _returnvalue "/Engine/EngineMeshes/Cube.Cube")
      (Rendering|SetCastShadow _returnvalue false)
      (Rendering|Material|SetMaterial _returnvalue 0 "/Game/Assets/Material/MI_Blue.MI_Blue"))))